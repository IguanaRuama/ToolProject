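; NPC actor Blueprint that runs cinematic item trades between the player and itself.
; An intro Level Sequence with runtime-rebound actors leads into a transfer menu widget, and closing it restores player camera and control.
; Transfers check the giver's owned and offered items against the receiver's wanted list, then update both inventories via message calls.
; A trade sequence then plays, reversed when the NPC receives, before looping back to the intro.
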(event Custom|onFinishedIntro
  (bind _returnvalue (Game|GetPlayerController 0))
  (bind _returnvalue_2 (UserInterface|CreateWidget "/Game/MyBlueprints/Widgets/WBO_TransferMenu.WBO_TransferMenu_C" _returnvalue))
  (bind _output_get (Variables|Default|SettradeWidget _returnvalue_2))
  (CallFunction|SetUIVariables _output_get)
  (UserInterface|Viewport|AddtoViewport _output_get 0)
  (Input|SetInputModeUIOnly _returnvalue _output_get "DoNotLock" false)
  (Variables|/Script/Engine.PlayerController|SetbShowMouseCursor _returnvalue true)
  (EventDispatchers|BindEventtoOnTransferComplete (Variables|Default|GettradeWidget) (delegate Custom|onTransferComplete)))

(event Custom|startTransfer
  (if (Utilities|IsValid (Variables|Default|Getintro))
    (CallFunction|PlayIntro (Variables|/Script/LevelSequence.LevelSequenceActor|GetSequencePlayer (Variables|Default|Getintro)))
    (else
      (bind (_outactor _returnvalue) (Sequencer|Player|CreateLevelSequencePlayer "/Game/MyBlueprints/LevelSequences/LS_Intro.LS_Intro"))
      (bind _output_get (Variables|Default|Setintro _outactor))
      (EventDispatchers|BindEventtoOnFinished _returnvalue (delegate Custom|onFinishedIntro))
      (CallFunction|PlayIntro _returnvalue))))

(event Custom|completeTransfer
  (if (Utilities|IsValid (Variables|Default|Gettrade))
    (CallFunction|PlayTrade (Variables|/Script/LevelSequence.LevelSequenceActor|GetSequencePlayer (Variables|Default|Gettrade)))
    (else
      (bind (_outactor _returnvalue) (Sequencer|Player|CreateLevelSequencePlayer "/Game/MyBlueprints/LevelSequences/LS_NPCGive.LS_NPCGive"))
      (Variables|Default|Settrade _outactor)
      (EventDispatchers|BindEventtoOnFinished _returnvalue (delegate Custom|onFinishedTrade))
      (bind _returnvalue_2 (Actor|GetActorOfClass "/Game/MyBlueprints/BP_TransferItem.BP_TransferItem_C"))
      (Class|BPIUpdateTransferItem|UpdateItem(Message) _returnvalue_2 (Variables|Default|GetselectedItem))
      (CallFunction|PlayTrade _returnvalue))))

(event Custom|onFinishedTrade
  (CallFunction|StartTransfer))

(event Custom|onTransferComplete
  (bind _returnvalue (Game|GetPlayerController 0))
  (Game|Player|SetViewTargetwithBlend (Game|GetPlayerController 0) (Game|GetPlayerCharacter 0) 0.0 "VTBlend_Linear" 0.0 false)
  (Pawn|Components|CharacterMovement|SetMovementMode (Variables|/Script/Engine.Character|GetCharacterMovement (Game|GetPlayerCharacter 0)) "MOVE_Walking" 0)
  (Input|SetInputModeGameOnly _returnvalue false)
  (Variables|/Script/Engine.PlayerController|SetbShowMouseCursor _returnvalue false)
  (Widget|RemovefromParent (Variables|Default|GettradeWidget)))

(event EventBeginPlay)

(event Collision|EventActorBeginOverlap
  (params (OtherActor :type Actor%20Object%20Reference)))

(event EventTick
  (params (DeltaSeconds :type Float%20%28single-precision%29)))

(event EventTryTransfer
  (params (item :type Object%20Object%20Reference))
  (bind _asbp_item_data_base (Utilities|Casting|CastToBP_ItemDataBase item))
  (bind _output_get (Variables|Default|SetselectedItem _asbp_item_data_base))
  (bind _result (CallFunction|CanGiveItem _output_get (Variables|Default|Getgiver) (Variables|Default|Getreciever)))
  (if _result
    (Class|BPITransferData|AlterInventory(Message) (Variables|Default|Getgiver) (Variables|Default|GetselectedItem) false)
    (Class|BPITransferData|AlterInventory(Message) (Variables|Default|Getreciever) (Variables|Default|GetselectedItem) true)
    (CallFunction|CompleteTransfer)))

(event EventSetTransferDirection
  (params (giver :type Actor%20Object%20Reference) (reciever :type Actor%20Object%20Reference))
  (Variables|Default|Setreciever reciever)
  (bind _output_get (Variables|Default|Setgiver giver))
  (bind _inventory (Class|BPITransferData|GetInventory(Message) _output_get))
  (bind _output_get_2 (Variables|Default|SetgiverInventoryRef _inventory))
  (Variables|Default|SetgiverItemsArray (Variables|/Game/MyBlueprints/AC_Inventory.AC_Inventory_C|GetownedItems _output_get_2))
  (bind _inventory_2 (Class|BPITransferData|GetInventory(Message) (Variables|Default|Getreciever)))
  (bind _output_get_3 (Variables|Default|SetrecieverInventoryRef _inventory_2))
  (Variables|Default|SetrecieverItemsArray (Variables|/Game/MyBlueprints/AC_Inventory.AC_Inventory_C|GetownedItems _output_get_3)))

(fn ConstructionScript)

(fn CanGiveItem
  (params (item :type BP%20Item%20Data%20Base%20Object%20Reference) (giver :type Actor%20Object%20Reference) (reciever :type Actor%20Object%20Reference))
  (bind _inventory (Class|BPITransferData|GetInventory(Message) giver))
  (bind _hasitem (Default|HasItem _inventory item))
  (Development|PrintString (Utilities|GetDisplayName item) true true "(R=1.000000,G=0.000000,B=0.906453,A=1.000000)")
  (Development|PrintString (Utilities|GetDisplayName giver) true true "(R=0.932196,G=0.006301,B=1.000000,A=1.000000)")
  (Development|PrintString (Utilities|GetDisplayName _inventory) true true "(R=1.000000,G=0.755225,B=0.000000,A=1.000000)")
  (for _array_element (Variables|/Game/MyBlueprints/AC_Inventory.AC_Inventory_C|GetofferedItems _inventory)
    (Development|PrintString (Utilities|GetDisplayName _array_element) true true "(R=1.000000,G=0.507347,B=0.000000,A=1.000000)"))
  (if (Utilities|Array|ContainsItem (Variables|/Game/MyBlueprints/AC_Inventory.AC_Inventory_C|GetofferedItems _inventory) item)
    (bind _inventory_2 (Class|BPITransferData|GetInventory(Message) reciever))
    (return (Math|Boolean|ANDBoolean _hasitem (Utilities|Array|ContainsItem (Variables|/Game/MyBlueprints/AC_Inventory.AC_Inventory_C|GetwantedItems _inventory_2) item) (Utilities|Array|ContainsItem (Variables|/Game/MyBlueprints/AC_Inventory.AC_Inventory_C|GetofferedItems _inventory) item)))))

(fn PlayIntro
  (params (sequence :type Level%20Sequence%20Player%20Object%20Reference))
  (CallFunction|SetIntroBindings (Variables|Default|Getintro))
  (bind _returnvalue (Actor|GetActorOfClass "/Script/CinematicCamera.CineCameraActor"))
  (Game|Player|SetViewTargetwithBlend (Game|GetPlayerController 0) _returnvalue 0.0 "VTBlend_Linear" 0.0 false)
  (Components|Timeline|SetPlaybackPosition sequence (Utilities|Struct|MakeMovieSceneSequencePlaybackParams "(FrameNumber=(Value=0),SubFrame=0.000000)" 0.0 "" "(Hours=0,Minutes=0,Seconds=0,Frames=0,Subframe=0.000000,bDropFrameFormat=False)" "Frame" "Play" false))
  (Sequencer|Player|Play sequence :!class /Script/MovieScene.MovieSceneSequencePlayer))

(fn SetIntroBindings
  (params (sequence :type Level%20Sequence%20Actor%20Object%20Reference))
  (bind _returnvalue (Class|LevelSequenceActor|GetSequence sequence))
  (Variables|/Script/LevelSequence.LevelSequenceActor|SetbOverrideInstanceData sequence true)
  (bind _returnvalue_2 (Class|MovieSceneSequenceExtensions|GetBindings _returnvalue))
  (for _array_element _returnvalue_2
    (bind _returnvalue_3 (Class|MovieSceneBindingExtensions|GetDisplayName _array_element))
    (switch string (Utilities|String|ToString(Text) _returnvalue_3)
      (:Player
        (bind _returnvalue_4 (Class|MovieSceneSequenceExtensions|GetBindingID _returnvalue _array_element))
        (Class|LevelSequenceActor|SetBinding (Variables|Default|Getintro) _returnvalue_4 (Utilities|Array|MakeArray (Variables|Default|GetplayerRef)) false))
      (:NPC
        (bind _returnvalue_5 (Class|MovieSceneSequenceExtensions|GetBindingID _returnvalue _array_element))
        (Class|LevelSequenceActor|SetBinding (Variables|Default|Getintro) _returnvalue_5 (Utilities|Array|MakeArray self) false)))))

(fn FilterInventory
  ;[0.15 0.15 0.15 0.5] Fix
  (Utilities|Array|Clear (Variables|Default|GetfilteredItemsArray))
  (for _array_element (Variables|Default|GetgiverItemsArray)
    (if (Utilities|Array|ContainsItem (Variables|Default|GetrecieverItemsArray) _array_element)
      (Utilities|Array|Add (Variables|Default|GetfilteredItemsArray) _array_element)))
  (return (Variables|Default|GetfilteredItemsArray)))

(fn HandleSelectedItem
  (params (selectedItem :type BP%20Item%20Data%20Base%20Object%20Reference))
  (Variables|Default|SetselectedItem selectedItem))

(fn PlayTrade
  (params (sequence :type Level%20Sequence%20Player%20Object%20Reference))
  (Widget|RemovefromParent (Variables|Default|GettradeWidget))
  (CallFunction|SetTradeBindings (Variables|Default|Gettrade))
  (if (== self (Variables|Default|Getgiver))
    (Sequencer|Player|Play sequence :!class /Script/MovieScene.MovieSceneSequencePlayer)
    (else
      (Class|MovieSceneSequencePlayer|PlayReverse sequence))))

(fn SetTradeBindings
  (params (sequence :type Level%20Sequence%20Actor%20Object%20Reference))
  (bind _returnvalue (Class|LevelSequenceActor|GetSequence sequence))
  (Variables|/Script/LevelSequence.LevelSequenceActor|SetbOverrideInstanceData sequence true)
  (bind _returnvalue_2 (Class|MovieSceneSequenceExtensions|GetBindings _returnvalue))
  (for _array_element _returnvalue_2
    (bind _returnvalue_3 (Class|MovieSceneBindingExtensions|GetDisplayName _array_element))
    (switch string (Utilities|String|ToString(Text) _returnvalue_3)
      (:Item
        (bind _returnvalue_4 (Class|MovieSceneSequenceExtensions|GetBindingID _returnvalue _array_element))
        (Class|LevelSequenceActor|SetBinding (Variables|Default|Gettrade) _returnvalue_4 (Utilities|Array|MakeArray (Variables|Default|GetspawnedItem)) false))
      (:NPC
        (bind _returnvalue_5 (Class|MovieSceneSequenceExtensions|GetBindingID _returnvalue _array_element))
        (Class|LevelSequenceActor|SetBinding (Variables|Default|Gettrade) _returnvalue_5 (Utilities|Array|MakeArray self) false)))))

(fn SetUIVariables
  (params (tradeWidget :type WBO%20Transfer%20Menu%20Object%20Reference))
  (Variables|/Game/MyBlueprints/Widgets/WBO_TransferMenu.WBO_TransferMenu_C|Setnpc tradeWidget self)
  (Variables|/Game/MyBlueprints/Widgets/WBO_TransferMenu.WBO_TransferMenu_C|SetnpcInventory tradeWidget (Variables|Default|GetInventory))
  (bind _output_get (Variables|/Game/MyBlueprints/Widgets/WBO_TransferMenu.WBO_TransferMenu_C|Setplayer tradeWidget (Game|GetPlayerCharacter 0)))
  (bind _inventory (Class|BPITransferData|GetInventory(Message) _output_get))
  (Variables|/Game/MyBlueprints/Widgets/WBO_TransferMenu.WBO_TransferMenu_C|SetplayerInventory tradeWidget _inventory))

(fn GetInventory
  (return 0))

(fn GetPlayerCamera)