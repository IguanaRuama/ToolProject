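; AC_Inventory is an inventory component that tracks an owner's items in three collections: owned, wanted and offered, which suggests a trading mechanic.
; Adding an item puts it in the owned collection and clears it from the wanted one.
; Removing an item only takes effect if it is offered, and then clears it from both owned and offered.
; HasItem reports whether an item is owned.
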(event Custom|removeItem
  (params (item :type BP%20Item%20Data%20Base%20Object%20Reference))
  (if (Utilities|Array|ContainsItem (Variables|Default|GetofferedItems) item)
    (Utilities|Array|RemoveItem (Variables|Default|GetownedItems) item)
    (Utilities|Array|RemoveItem (Variables|Default|GetofferedItems) item)))

(event Custom|addItem
  (params (item :type BP%20Item%20Data%20Base%20Object%20Reference))
  (Utilities|Array|Add (Variables|Default|GetownedItems) item)
  (if (Utilities|Array|ContainsItem (Variables|Default|GetwantedItems) item)
    (Utilities|Array|RemoveItem (Variables|Default|GetwantedItems) item)))

(event EventBeginPlay)

(event EventTick
  (params (DeltaSeconds :type Float%20%28single-precision%29)))

(fn HasItem
  (params (item :type BP%20Item%20Data%20Base%20Object%20Reference))
  (return (Utilities|Array|ContainsItem (Variables|Default|GetownedItems) item)))